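; Tank Blueprint for a player-controlled tank with an orbiting aim camera and a cannon.
; On BeginPlay it passes its Barrel and TankTurret components to inherited setters.
; Aim axes rotate the AzimuthGimbal in yaw and the SpringArm in pitch, scaled by delta time for frame-rate independence.
; The Fire action calls FireCannon, whose logic lives outside this Blueprint.
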(event `self.ReceiveBeginPlay`
  (`self.SetBarrelReference` (`self.Barrel`))
  (`self.SetTurretReference` (`self.TankTurret`)))

(event `InputAxis|AimAzimuth`
  (params (AxisValue :type "Float (single-precision)"))
  ;[1 1 1] Handle Horizontal Camera Input
  (`SceneComponent.K2_AddLocalRotation` (`self.Azimuth Gimbal`) (`KismetMathLibrary.MakeRotator` 0.0 0.0 (* AxisValue (`GameplayStatics.GetWorldDeltaSeconds`) 75.0)) false false))

(event `InputAxis|AimElevation`
  (params (AxisValue :type "Float (single-precision)"))
  ;[1 1 1] Handle Vertical Camera Input
  (`SceneComponent.K2_AddLocalRotation` (`self.SpringArm`) (`KismetMathLibrary.MakeRotator` 0.0 (* AxisValue (`GameplayStatics.GetWorldDeltaSeconds`) 75.0)) false false))

(event `InputAction|Fire`
  (params (Key :type "Key Structure"))
  ;[1 1 1] Firing the Cannon
  (:`Pressed`
    (`self.FireCannon`)))

(fn `UserConstructionScript`)